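; BP_FallingRockSpawner repeatedly spawns BP_RockProjectile actors at the transform of its Sphere component.
; On BeginPlay it hides the Sphere and disables its collision, leaving it as an invisible spawn marker.
; Tick drives a random Delay of whole seconds, which acts as the spawn timer because it ignores re-triggers while pending.
; Each spawned rock gets a fixed life span so it cleans itself up.
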(event EventBeginPlay
  (bind _sphere (Variables|Default|GetSphere))
  (Rendering|SetVisibility _sphere false false)
  (Collision|SetCollisionEnabled _sphere "NoCollision"))

(event Collision|EventActorBeginOverlap
  (params (OtherActor :type Actor%20Object%20Reference)))

(event EventTick
  (params (DeltaSeconds :type Float%20%28single-precision%29))
  (Utilities|FlowControl|Delay (Math|Conversions|ToFloat(Integer) (+ (Math|Random|RandomInteger 4) 1)))
  (bind _returnvalue (Game|SpawnActorfromClass "/Game/UsedAssets/Blueprints/BP_RockProjectile.BP_RockProjectile_C" (Transformation|GetWorldTransform (Variables|Default|GetSphere)) "Undefined" 0 0))
  (Actor|SetLifeSpan _returnvalue 7.0))

(fn ConstructionScript)